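; BoxStove_BP is a stove actor that shows a UI widget while something overlaps it.
; On begin overlap it creates a HUDClass widget for player 0 and adds it to the viewport; on end overlap it removes all widgets, not just its own.
; Both events require player 0's HUD to be HUD_BP, and neither checks which actor overlapped.
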(event Collision|EventActorBeginOverlap
  (params (OtherActor :type Actor%20Object%20Reference))
  (Utilities|Casting|CastToHUD_BP (HUD|GetHUD (Game|GetPlayerController 0)))
  (bind _returnvalue (UserInterface|CreateWidget (Variables|Default|GetHUDClass) (Game|GetPlayerController 0)))
  (UserInterface|Viewport|AddtoViewport _returnvalue 0))

(event Collision|EventActorEndOverlap
  (params (OtherActor :type Actor%20Object%20Reference))
  (Utilities|Casting|CastToHUD_BP (HUD|GetHUD (Game|GetPlayerController 0)))
  (Viewport|RemoveAllWidgets))

(fn ConstructionScript)