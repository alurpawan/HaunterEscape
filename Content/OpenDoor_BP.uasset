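; OpenDoor_BP is a trigger actor that lets the player open a referenced Door once the Key actor is hidden.
; On overlap it shows a HUD widget, swapping it for an open-door prompt and enabling input if the Key is hidden.
; The Open action plays a timeline that adds curve-driven yaw to the door's rotation, then destroys the trigger.
; Ending the overlap removes all widgets and disables input.
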(event Collision|EventActorBeginOverlap
  (params (OtherActor :type Actor%20Object%20Reference))
  (Utilities|Casting|CastToHUD_BP (HUD|GetHUD (Game|GetPlayerController 0)))
  (bind _returnvalue (UserInterface|CreateWidget (Variables|Default|GetHUDClass) (Game|GetPlayerController 0)))
  (UserInterface|Viewport|AddtoViewport _returnvalue 0)
  (bind _asactor (Utilities|Casting|CastToActor (Variables|Default|GetKey)))
  (if (Variables|/Script/Engine.Actor|GetbHidden _asactor)
    (Widget|RemovefromParent _returnvalue)
    (bind _returnvalue_2 (UserInterface|CreateWidget "/Game/MyHUD/OpenDoorHUD.OpenDoorHUD_C"))
    (UserInterface|Viewport|AddtoViewport _returnvalue_2 0)
    (Input|EnableInput (Game|GetPlayerController 0))))

(event Collision|EventActorEndOverlap
  (params (OtherActor :type Actor%20Object%20Reference))
  (Utilities|Casting|CastToHUD_BP (HUD|GetHUD (Game|GetPlayerController 0)))
  (Viewport|RemoveAllWidgets)
  (Input|DisableInput (Game|GetPlayerController 0)))

(event Input|ActionEvents|InputActionOpen
  (params (Key :type Key%20Structure))
  (:Pressed
    (Variables|Default|SetInit_Rot (Transformation|GetActorRotation (Variables|Default|GetDoor)))
    (bind _doorcurve (Timeline|OpenDoor Play)
      (:Update
        (Transformation|SetActorRotation (Variables|Default|GetDoor) (Math|Rotator|CombineRotators (Variables|Default|GetInit_Rot) (Math|Rotator|MakeRotator 0.0 0.0 _doorcurve))))
      (:Finished
        (Actor|DestroyActor)))))

(fn ConstructionScript)