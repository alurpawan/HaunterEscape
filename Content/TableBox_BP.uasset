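; TableBox_BP is an interactive table drawer that slides open to reveal a key.
; Overlap with the actor adds a TestHUD prompt widget, enables input and sets IsInBox, which gates the Open action; leaving clears the flag and removes all widgets.
; Open toggles the drawer by an instant Y offset, carrying KeyActor along when opening.
; Closing hides the key and prints a pickup message, with no inventory state recorded.
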(event Collision|EventActorBeginOverlap
  (params (OtherActor :type Actor%20Object%20Reference))
  ;[1 1 1] Display message on screen
  (Utilities|Casting|CastToHUD_BP (HUD|GetHUD (Game|GetPlayerController 0)))
  (bind _returnvalue (UserInterface|CreateWidget "/Game/MyHUD/TestHUD.TestHUD_C" (Game|GetPlayerController 0)))
  (UserInterface|Viewport|AddtoViewport _returnvalue 0)
  (Variables|Default|SetIsInBox true)
  (Input|EnableInput (Game|GetPlayerController 0)))

(event Collision|EventActorEndOverlap
  (params (OtherActor :type Actor%20Object%20Reference))
  ;[1 1 1] Display message on screen
  (Utilities|Casting|CastToHUD_BP (HUD|GetHUD (Game|GetPlayerController 0)))
  (Viewport|RemoveAllWidgets)
  (Variables|Default|SetIsInBox false))

(event Input|ActionEvents|InputActionOpen
  (params (Key :type Key%20Structure))
  (bind _keyactor (Variables|Default|GetKeyActor))
  ;[1 1 1] Check Is Open Pressed
  (:Pressed
    (if (Variables|Default|GetIsInBox)
      (if (Variables|Default|GetIsOpen)
        ;[1 1 1] Close Drawer
        (Transformation|SetActorLocation (+ (Transformation|GetActorLocation) "0,-30.000000,0.000000") false false)
        (Variables|Default|SetIsOpen false)
        (Rendering|SetActorHiddenInGame (Variables|Default|GetKeyActor) true)
        (Development|PrintText "You have obtained Key")
        (else
          ;[1 1 1] Open Drawer
          (Transformation|SetActorLocation (+ (Transformation|GetActorLocation) "0,30.000000,0.000000") false false)
          (Variables|Default|SetIsOpen true)
          (Transformation|SetActorLocation _keyactor (+ (Transformation|GetActorLocation _keyactor) "0,30.000000,0.000000") false false))))))

(fn ConstructionScript)